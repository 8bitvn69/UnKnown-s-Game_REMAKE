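; Player-controlled physics ball that rolls, jumps and carries an orbit camera.
; The Scene component uses absolute rotation and scale, with look input yawing it and pitching the SpringArm within angle limits.
; Movement applies mass-independent torque to BallMesh around the Arrow's axes, and jump applies a vertical velocity impulse.
; Both work only while grounded, a flag set by hitting "Ground"-tagged actors and cleared only on jumping.
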(event `self.ReceiveBeginPlay`
  (`SceneComponent.SetAbsolute` (`self.Scene`) false true true))

(event `self.ReceiveHit`
  (params (MyComp :type "PrimitiveComponent Object Reference") (Other :type "Actor Object Reference") (OtherComp :type "PrimitiveComponent Object Reference") (bSelfMoved :type Boolean) (HitLocation :type "Vector Structure") (HitNormal :type "Vector Structure") (NormalImpulse :type "Vector Structure") (Hit :type "HitResult Structure (by ref)"))
  (if (`self.ActorHasTag` Other "Ground")
    (set `self.IsOnTheGround` true)))

(event `InputAxis|Horizontal`
  (params (AxisValue :type "Float (single-precision)"))
  ;[1 1 1] Setup Camera
  (`SceneComponent.K2_AddRelativeRotation` (`self.Scene`) (`KismetMathLibrary.MakeRotator` 0.0 0.0 (* AxisValue 2.0)) false false))

(event `InputAxis|Vertical`
  (params (AxisValue :type "Float (single-precision)"))
  (bind _returnvalue (* AxisValue 2.0))
  (bind _springarm (`self.SpringArm`))
  (bind _returnvalue_2 (+ _returnvalue (.pitch (`SceneComponent.RelativeRotation` _springarm))))
  ;[1 1 1] Setup Camera
  (if (and (> _returnvalue_2 (`self.MinAngle`)) (< _returnvalue_2 (`self.MaxAngle`)))
    (`SceneComponent.K2_AddRelativeRotation` _springarm (`KismetMathLibrary.MakeRotator` 0.0 _returnvalue) false false)))

(event `InputAxis|MoveForward`
  (params (AxisValue :type "Float (single-precision)"))
  ;[1 1 1] Setup Movement
  (if (`self.IsOnTheGround`)
    (`PrimitiveComponent.AddTorque` (`self.BallMesh`) (* (`SceneComponent.GetRightVector` (`self.Arrow`)) (* AxisValue 50.0)) "None" true)))

(event `InputAxis|MoveRight`
  (params (AxisValue :type "Float (single-precision)"))
  ;[1 1 1] Setup Movement
  (if (`self.IsOnTheGround`)
    (`PrimitiveComponent.AddTorque` (`self.BallMesh`) (* (`SceneComponent.GetForwardVector` (`self.Arrow`)) (* AxisValue -50.0)) "None" true)))

(event `InputAction|Jump`
  (params (Key :type "Key Structure"))
  ;[1 1 1] Setup Movement
  (:`Pressed`
    (if (`self.IsOnTheGround`)
      (`PrimitiveComponent.AddImpulse` (`self.BallMesh`) (0.0 0.0 500.0) "None" true)
      (set `self.IsOnTheGround` false))))

(fn `UserConstructionScript`)